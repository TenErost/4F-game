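; BP_Skeleton is a damageable 2D skeleton enemy with a widget health bar.
; Health queries, healing and damage forward to BPCDamageSystem, whose damage-response and death events are bound in the Construction Script.
; Death sets IsDead, plays a PaperZD override animation and destroys the actor after a delay, while damage responses only print.
; Player chasing is unwired, and UpdateAnimation, which swaps player idle/run flipbooks by velocity, is not called here.
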(event Custom|Death
  ;[0.15 0.15 0.15 0.5] Death
  (Development|PrintString "Died")
  (Variables|Default|SetIsDead true)
  (|PlayAnimationOverridewithCallbacks (Variables|/Script/PaperZD.PaperZDAnimationComponent|GetAnimInstance (Variables|Default|GetAnimationComponent)) "/Game/Blueprints/Damage_System/Enemy/Skeleton/AnimSequences/Death.Death" "DefaultSlot" 1.0 0.0
    (:then
      _)
    (:OnCompleted
      _))
  (Utilities|FlowControl|Delay 1e+01)
  (Actor|DestroyActor))

(event Custom|DamageResponse
  (params (DamageResponse :type E_DamageResponse%20Enum :default "NewEnumerator0"))
  ;[0.15 0.15 0.15 0.5] DamageResponse
  (Development|PrintString (Utilities|String|EnumtoString DamageResponse)))

(event EventBeginPlay
  ;[0.15 0.15 0.15 0.5] Health Bar creation
  (bind _returnvalue (UserInterface|CreateWidget "/Game/UI/W_HealthBar.W_HealthBar_C" 0 self))
  (UserInterface|SetWidget (Variables|Default|GetWidget) _returnvalue))

(event Collision|EventActorBeginOverlap
  (params (OtherActor :type Actor%20Object%20Reference)))

(event EventTick
  (params (DeltaSeconds :type Float%20%28single-precision%29))
  ;[0.15 0.15 0.15 0.5] Chase Player
)

(fn ConstructionScript
  (bind _bpc_damagesystem (Variables|Default|GetBPC_DamageSystem))
  (EventDispatchers|BindEventtoOnDeath _bpc_damagesystem (EventDispatchers|CreateEvent :!event Custom|Death))
  (EventDispatchers|BindEventtoOnDamageResponse _bpc_damagesystem (EventDispatchers|CreateEvent :!event Custom|DamageResponse)))

(fn UpdateAnimation
  (if (<= (Math|Vector|VectorLength (Transformation|GetVelocity)) 0.0)
    (Sprite|SetFlipbook (Variables|Default|GetSprite) "/Game/PaperAssets/Player/Flipbooks/FB_Player_Idle.FB_Player_Idle")
    (else
      (Sprite|SetFlipbook (Variables|Default|GetSprite) "/Game/PaperAssets/Player/Flipbooks/FB_Player_Run.FB_Player_Run"))))

(fn GetCurrentHealth
  (return (Variables|/Game/Blueprints/Damage_System/BPC_DamageSystem.BPC_DamageSystem_C|GetHealth (Variables|Default|GetBPC_DamageSystem))))

(fn GetMaxHealth
  (return (Variables|/Game/Blueprints/Damage_System/BPC_DamageSystem.BPC_DamageSystem_C|GetMaxHealth (Variables|Default|GetBPC_DamageSystem))))

(fn Heal
  (params (Amount :type Float%20%28double-precision%29))
  (bind _newhealth (Default|Heal (Variables|Default|GetBPC_DamageSystem) Amount))
  (return _newhealth))

(fn TakeDamage
  (params (DamageInfo :type S%20Damage%20Info%20Structure))
  (bind _wasdamaged (Default|TakeDamage (Variables|Default|GetBPC_DamageSystem) DamageInfo))
  (return _wasdamaged))