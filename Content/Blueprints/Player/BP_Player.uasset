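; Player character with flipbook sprite, Enhanced Input movement, jump, interact, pause menu and debug slime spawning.
; Attack plays an animation override that blocks moving and jumping, while a forward sphere trace damages and launches the hit character.
; BPCDamageSystem handles health, exposed through damage and heal wrapper functions and shown in a health bar widget.
; Death and damage responses only print messages.
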(event Custom|Death
  ;[0.15 0.15 0.15 0.5] Death
  (Development|PrintString "PlayerDied"))

(event Custom|DamageResponse
  (params (DamageResponse :type E_DamageResponse%20Enum :default "NewEnumerator0"))
  ;[0.15 0.15 0.15 0.5] Damage Response
  (Development|PrintString (Utilities|String|EnumtoString DamageResponse)))

(event Input|EnhancedActionEvents|EnhancedInputActionIA_Move
  (params (ActionValue :type Vector%202D%20Structure) (ElapsedSeconds :type Float%20%28double-precision%29) (TriggeredSeconds :type Float%20%28double-precision%29) (InputAction :type Input%20Action%20Object%20Reference :default "/Game/Input/Actions/IA_Move.IA_Move"))
  (bind (_x _y) (Math|Vector2D|BreakVector2D ActionValue))
  ;[0.15 0.15 0.15 0.5] Moving
  (if (not (Variables|Default|GetIsAttacking))
    (Pawn|Input|AddMovementInput "1.000000,0.000000,0.000000" _x false)
    (Pawn|Input|AddMovementInput "0.000000,1.000000,0.000000" _y false)
    (Math|Float|CompareFloat _x 0.0
      (:>
        (bind _output_get (Variables|Default|SetPlayerRotation "0, 0, 0"))
        (Transformation|SetActorRotation _output_get))
      (:<
        (bind _output_get_2 (Variables|Default|SetPlayerRotation "0.000000,180.000000,0.000000"))
        (Transformation|SetActorRotation _output_get_2)))))

(event Input|EnhancedActionEvents|EnhancedInputActionIA_Jump
  (params (ActionValue :type Boolean) (ElapsedSeconds :type Float%20%28double-precision%29) (TriggeredSeconds :type Float%20%28double-precision%29) (InputAction :type Input%20Action%20Object%20Reference :default "/Game/Input/Actions/IA_Jump.IA_Jump"))
  ;[0.15 0.15 0.15 0.5] Action: Jump
  (:Started
    (if (not (Variables|Default|GetIsAttacking))
      (Character|Jump)))
  (:Completed
    (Character|StopJumping)))

(event Input|EnhancedActionEvents|EnhancedInputActionIA_Attack
  (params (ActionValue :type Boolean) (ElapsedSeconds :type Float%20%28double-precision%29) (TriggeredSeconds :type Float%20%28double-precision%29) (InputAction :type Input%20Action%20Object%20Reference :default "/Game/Input/Actions/IA_Attack.IA_Attack"))
  (bind (_returnvalue _returnvalue2 _array) (|TraceSearch))
  ;[0.15 0.15 0.15 0.5] Action: Attack
  (:Started
    (if (not (Variables|Default|GetIsAttacking))
      (|PlayAnimationOverridewithCallbacks (Variables|/Script/PaperZD.PaperZDAnimationComponent|GetAnimInstance (Variables|Default|GetAnimationComponent)) "/Game/Blueprints/Player/AnimSequences/Attack.Attack" "DefaultSlot" 1.0 0.0
        (:then
          (Variables|Default|SetIsAttacking true)
          (bind _outhit (Collision|SphereTraceForObjects _returnvalue _returnvalue2 3e+01 _array false 0 "ForDuration" true "(R=1.000000,G=0.000000,B=0.000000,A=1.000000)" "(R=0.000000,G=1.000000,B=0.000000,A=1.000000)" 1.0))
          (if true
            (Class|BPIDamagable|TakeDamage(Message) (.HitActor (Collision|BreakHitResult _outhit)) (Utilities|Struct|MakeS_DamageInfo 1.0 "NewEnumerator1" "NewEnumerator4"))
            (bind _ascharacter (Utilities|Casting|CastToCharacter (.HitActor (Collision|BreakHitResult _outhit))))
            (Character|LaunchCharacter _ascharacter (Math|Vector|MakeVector (+ (.X (Math|Vector|BreakVector (Math|Vector|GetUnitDirection(Vector) _returnvalue2 (Transformation|GetActorLocation (.HitActor (Collision|BreakHitResult _outhit)))))) 4e+02) (.Y (Math|Vector|BreakVector (Math|Vector|GetUnitDirection(Vector) _returnvalue2 (Transformation|GetActorLocation (.HitActor (Collision|BreakHitResult _outhit)))))) (+ (.Z (Math|Vector|BreakVector (Math|Vector|GetUnitDirection(Vector) _returnvalue2 (Transformation|GetActorLocation (.HitActor (Collision|BreakHitResult _outhit)))))) 6e+02)) true true)))
        (:OnCompleted
          (Variables|Default|SetIsAttacking false :!label _label))
        (:OnCancelled
          (goto _label))))))

(event Input|EnhancedActionEvents|EnhancedInputActionIA_Pause
  (params (ActionValue :type Boolean) (ElapsedSeconds :type Float%20%28double-precision%29) (TriggeredSeconds :type Float%20%28double-precision%29) (InputAction :type Input%20Action%20Object%20Reference :default "/Game/Input/Actions/IA_Pause.IA_Pause"))
  (bind _returnvalue (Game|GetPlayerController 0))
  (bind _returnvalue_2 (Game|GetPlayerController 0))
  ;[0.15 0.15 0.15 0.5] Action: Pause
  (:Started
    (if (not (Game|IsGamePaused))
      (Game|SetGamePaused true)
      (bind _returnvalue_3 (UserInterface|CreateWidget "/Game/UI/Menu/UWB_PauseMenu.UWB_PauseMenu_C"))
      (UserInterface|Viewport|AddtoViewport _returnvalue_3 0)
      (Variables|/Script/Engine.PlayerController|SetbShowMouseCursor _returnvalue true)
      (Input|SetInputModeGameandUI _returnvalue 0 "LockInFullscreen" true false)
      (else
        (Game|SetGamePaused false)
        (Widget|RemovefromParent _returnvalue_3)
        (Variables|/Script/Engine.PlayerController|SetbShowMouseCursor _returnvalue_2 false)
        (Input|SetInputModeGameOnly _returnvalue_2 false)))))

(event Input|EnhancedActionEvents|EnhancedInputActionIA_Use
  (params (ActionValue :type Boolean) (ElapsedSeconds :type Float%20%28double-precision%29) (TriggeredSeconds :type Float%20%28double-precision%29) (InputAction :type Input%20Action%20Object%20Reference :default "/Game/Input/Actions/IA_Use.IA_Use"))
  ;[0.15 0.15 0.15 0.5] Interact
  (:Started
    (bind _array_element (Utilities|Array|ForEachLoopwithBreak (Collision|GetOverlappingActors 0 :!class /Script/Engine.Actor) :!label _label)
      (:LoopBody
        (if (Utilities|DoesObjectImplementInterface _array_element "/Game/Blueprints/BPI_Interact.BPI_Interact_C")
          (Class|BPIInteract|Interact(Message) _array_element)
          (goto _label Break))))))

(event Input|EnhancedActionEvents|EnhancedInputActionIA_SpawnSlime
  (params (ActionValue :type Boolean) (ElapsedSeconds :type Float%20%28double-precision%29) (TriggeredSeconds :type Float%20%28double-precision%29) (InputAction :type Input%20Action%20Object%20Reference :default "/Game/Input/Actions/IA_SpawnSlime.IA_SpawnSlime"))
  ;[0.15 0.15 0.15 0.5] Spawn slime on L press
  (:Started
    (Actor|GetActorOfClass "/Game/Blueprints/Damage_System/Enemy/BP_Enemy1.BP_Enemy1_C")
    (Game|SpawnActorfromClass "/Game/Blueprints/Damage_System/Enemy/BP_Enemy1.BP_Enemy1_C" (Transformation|GetActorTransform self) "Undefined" "MultiplyWithRoot" 0 0)))

(event EventBeginPlay
  ;[0.15 0.15 0.15 0.5] Map controller
  (Utilities|FlowControl|Sequence
    (:then_0
      (bind _asplayer_controller (Utilities|Casting|CastToPlayerController (Pawn|GetController)))
      (Input|AddMappingContext (PlayerController|LocalPlayerSubsystems|GetEnhancedInputLocalPlayerSubsystem _asplayer_controller) "/Game/Input/IMC_Hybrid.IMC_Hybrid" 0 "(bIgnoreAllPressedKeysUntilRelease=True,bForceImmediately=False,bNotifyUserSettings=False)"))
    (:then_1
      (bind _returnvalue (UserInterface|CreateWidget "/Game/UI/W_HealthBar.W_HealthBar_C" 0 self))
      (UserInterface|SetWidget (Variables|Default|GetWidget) _returnvalue))))

(event Collision|EventActorBeginOverlap
  (params (OtherActor :type Actor%20Object%20Reference)))

(event EventTick
  (params (DeltaSeconds :type Float%20%28single-precision%29)))

(fn ConstructionScript
  (bind _bpc_damagesystem (Variables|Default|GetBPC_DamageSystem))
  (EventDispatchers|BindEventtoOnDeath _bpc_damagesystem (EventDispatchers|CreateEvent :!event Custom|Death))
  (EventDispatchers|BindEventtoOnDamageResponse _bpc_damagesystem (EventDispatchers|CreateEvent :!event Custom|DamageResponse)))

(fn UpdateAnimation
  (if (<= (Math|Vector|VectorLength (Transformation|GetVelocity)) 0.0)
    (Sprite|SetFlipbook (Variables|Default|GetSprite) "/Game/PaperAssets/Player/Flipbooks/FB_Player_Idle.FB_Player_Idle")
    (else
      (Sprite|SetFlipbook (Variables|Default|GetSprite) "/Game/PaperAssets/Player/Flipbooks/FB_Player_Run.FB_Player_Run"))))

(fn GetCurrentHealth
  (return (Variables|/Game/Blueprints/Damage_System/BPC_DamageSystem.BPC_DamageSystem_C|GetHealth (Variables|Default|GetBPC_DamageSystem))))

(fn GetMaxHealth
  (return (Variables|/Game/Blueprints/Damage_System/BPC_DamageSystem.BPC_DamageSystem_C|GetMaxHealth (Variables|Default|GetBPC_DamageSystem))))

(fn Heal
  (params (Amount :type Float%20%28double-precision%29))
  (bind _newhealth (Default|Heal (Variables|Default|GetBPC_DamageSystem) Amount))
  (return _newhealth))

(fn TakeDamage
  (params (DamageInfo :type S%20Damage%20Info%20Structure))
  (bind _wasdamaged (Default|TakeDamage (Variables|Default|GetBPC_DamageSystem) DamageInfo))
  (return _wasdamaged))